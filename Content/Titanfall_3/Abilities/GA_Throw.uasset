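; Grenade-throw Gameplay Ability that previews the trajectory while input is held and throws on release.
; A looping timer refreshes the locally controlled player's predicted path, feeding a Niagara arc and placing an impact decal.
; Lethal grenades cook while held, setting the fuse and applying a self-damage effect if held too long.
; The authority spawns the grenade and launches it along control rotation; ending the ability hides the arc and commits cooldown.
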(event `self.K2_ActivateAbility`
  (bind _arcspawn (`/Game/Titanfall_3/GameData/BP_ShooterCharacter.ArcSpawn` (cast `/Game/Titanfall_3/GameData/BP_ShooterCharacter` (`self.GetAvatarActorFromActorInfo`) :!pure true)))
  (bind _returnvalue (`NiagaraFunctionLibrary.SpawnSystemAttached` "/Game/Titanfall_3/VFX/Arc/NS_Arc.NS_Arc" _arcspawn "None" (`SceneComponent.K2_GetComponentLocation` _arcspawn) (struct) "KeepWorldPosition"))
  (set `self.Arc` _returnvalue)
  (`KismetSystemLibrary.K2_SetTimerDelegate` (`|CreateDelegate` :!event `ArcSpawn`) 0.1 true)
  (if (`self.bLethal`)
    (set `self.CookTime` (`KismetSystemLibrary.GetGameTimeInSeconds`))
    (bind _returnvalue_2 (`KismetSystemLibrary.K2_SetTimerDelegate` (`|CreateDelegate` :!event `ExplodeSelf`) (`self.MaxCookTime`)))
    (set `self.ExplodeTimer` _returnvalue_2))
  (`AbilityTask_WaitInputRelease.WaitInputRelease` false
    (:`OnRelease`
      (`self.ThrowNade`))))

(event `ThrowNade`
  (bind _returnvalue (`self.GetAvatarActorFromActorInfo`))
  (`KismetSystemLibrary.K2_ClearAndInvalidateTimerHandle` (`self.ExplodeTimer`))
  (`self.K2_HasAuthority`
    (:`True`
      (bind _returnvalue_2 (`|SpawnActorFromClass` (`self.Grenade Class`) (`KismetMathLibrary.MakeTransform` (`Actor.K2_GetActorLocation` _returnvalue) (`Actor.K2_GetActorRotation` _returnvalue)) "Undefined" "MultiplyWithRoot" null (`self.RemainingCookTime`) (cast `AirShooterCharacter` _returnvalue :!pure true)))
      (`/Game/Titanfall_3/BPs/BP_Nade.Thow Impulse` _returnvalue_2 (`self.GetThrowSpeed`))
      (`self.K2_EndAbility`))))

(event `self.K2_OnEndAbility`
  (params (bWasCancelled :type Boolean))
  (`ActorComponent.Deactivate` (`self.Arc`))
  (`self.K2_CommitAbilityCooldown` false))

(event `ExplodeSelf`
  (`self.BP_ApplyGameplayEffectToOwner` "/Game/Titanfall_3/Abilities/Effects/GE_NadeSelf.GE_NadeSelf_C")
  (`KismetSystemLibrary.Delay` 0.2)
  (`self.K2_EndAbility`))

(event `ArcSpawn`
  (bind _vectorarray (`self.VectorArray`))
  (if (`Pawn.IsLocallyControlled` (cast `AirShooterCharacter` (`self.GetAvatarActorFromActorInfo`) :!pure true))
    (bind _predictresult (`GameplayStatics.Blueprint_PredictProjectilePath_Advanced` (make `PredictProjectilePathParams` (`SceneComponent.K2_GetComponentLocation` (`/Game/Titanfall_3/GameData/BP_ShooterCharacter.ArcSpawn` (cast `/Game/Titanfall_3/GameData/BP_ShooterCharacter` (`self.GetAvatarActorFromActorInfo`) :!pure true))) (`self.GetThrowSpeed`))))
    (`KismetArrayLibrary.Array_Clear` (`self.VectorArray`))
    (for _array_element (`.PathData` (break `PredictProjectilePathResult` _predictresult))
      (`KismetArrayLibrary.Array_Add` (`self.VectorArray`) (`.Location` (break `PredictProjectilePathPointData` _array_element))))
    (`NiagaraDataInterfaceArrayFunctionLibrary.SetNiagaraArrayPosition` (`self.Arc`) "Position2" _vectorarray)
    (`GameplayStatics.SpawnDecalAtLocation` "/Game/Titanfall_3/VFX/Arc/MI_DecalAim_Inst.MI_DecalAim_Inst" (20.0 20.0 20.0) (`|GetArrayItem` _vectorarray (`KismetArrayLibrary.Array_LastIndex` _vectorarray)) (`KismetMathLibrary.MakeRotFromX` (* (`.ImpactNormal` (`GameplayStatics.BreakHitResult` (`.HitResult` (break `PredictProjectilePathResult` _predictresult)))) -1.0)) 0.1)))

(fn `GetThrowSpeed`
  (returns (ReturnValue :type "Vector Structure"))
  (return (* (`KismetMathLibrary.GetForwardVector` (`KismetMathLibrary.MakeRotator` 0.0 (.pitch (`Controller.GetControlRotation` (cast `PlayerController` (`Pawn.GetController` (`self.GetOwningCharacter`)) :!pure true))) (.yaw (`Controller.GetControlRotation` (cast `PlayerController` (`Pawn.GetController` (`self.GetOwningCharacter`)) :!pure true))))) (`self.ThrowSpeed`))))

(fn `RemainingCookTime`
  (returns (CookTime :type "Float (double-precision)"))
  (bind _returnvalue (- (`KismetSystemLibrary.GetGameTimeInSeconds`) (`self.CookTime`)))
  (if (`self.bLethal`)
    (return (`KismetMathLibrary.FMax` _returnvalue (- (`self.MaxCookTime`) _returnvalue)))
    (else
      (return 3.0))))