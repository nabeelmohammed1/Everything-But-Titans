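; Gameplay ability for the player's jump and double jump, run on the locally controlled client.
; Activation performs the first jump, then waits for a jump gameplay event to double jump with boosted Z velocity unless cooldown-tagged, ending upon landing in Walking mode.
; Ending after a double jump applies a cooldown effect with a SetByCaller duration.
; A DirectionalJumping helper computes momentum-preserving air-boost velocity, but the event graph never calls it.
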(event `self.K2_OnEndAbility`
  (params (bWasCancelled :type Boolean))
  (if (> (`self.JumpCount`) 1)
    (set `self.JumpCount` 0)
    (set `self.JumpCooldown` 1.5)
    (bind _returnvalue (`AbilitySystemBlueprintLibrary.AssignTagSetByCallerMagnitude` (`self.MakeOutgoingGameplayEffectSpec` "/Game/Titanfall_3/Abilities/Effects/GE_JumpCooldown.GE_JumpCooldown_C") (struct :`TagName` "Data.Jump.Cooldown") (`self.JumpCooldown`)))
    (`self.K2_ApplyGameplayEffectSpecToOwner` _returnvalue)
    (else
      (set `self.JumpCount` 0))))

(event `self.K2_ActivateAbility`
  (bind _returnvalue (`self.GetOwningCharacter`))
  (`self.IsLocallyControlled`
    (:`True`
      (`self.K2_CommitAbility`)
      (if (`NavMovementInterface.IsFalling` (`self.GetCharacterMovement`))
        (`Character.Jump` _returnvalue)
        (set `self.JumpCount` 1)
        (else
          (`Character.Jump` _returnvalue)
          (`KismetSystemLibrary.PrintString` "1st Jump")
          (set `self.JumpCount` 1)))
      (`KismetSystemLibrary.Delay` 0.2)
      (`AbilityTask_WaitGameplayEvent.WaitGameplayEvent` (struct :`TagName` "Event.ActivateAbility.Jump") null
        (:`then`
          (`AbilityTask_WaitMovementModeChange.CreateWaitMovementModeChange` "MOVE_Walking"
            (:`OnChange`
              (`KismetSystemLibrary.PrintString` "landed")
              (`self.K2_EndAbility`))))
        (:`EventReceived`
          (`KismetSystemLibrary.PrintString` "double jump time" true true (struct :`R` 1.0 :`G` 0.033357 :`A` 1.0))
          (bind _returnvalue_2 (message `GameplayTagAssetInterface.HasMatchingGameplayTag` (`AbilitySystemBlueprintLibrary.GetAbilitySystemComponent` (`self.GetAvatarActorFromActorInfo`)) (struct :`TagName` "Cooldown.Jump")))
          (if _returnvalue_2
            (`KismetSystemLibrary.PrintString` "i shouldnt be jumping")
            (elif (< (`self.JumpCount`) 2)
              (set `CharacterMovementComponent.JumpZVelocity` (`self.DoubleJumpVel`) (`self.GetCharacterMovement`))
              (`Character.Jump` (`self.GetOwningCharacter`))
              (set `self.JumpCount` 2)
              (`KismetSystemLibrary.PrintString` "double jumped")
              (else
                (`KismetSystemLibrary.PrintString` "no 3td jump buddy" true true (struct :`R` 0.893212 :`G` 0.329236 :`B` 1.0 :`A` 1.0))))))))))

(fn `DirectionalJumping`
  (returns (ReturnValue :type "Vector Structure"))
  (locals (OldVel :type "Vector Structure" :default (0.0 0.0 0.0)))
  (set `local.OldVel` (`MovementComponent.Velocity` (`self.GetCharacterMovement`)))
  (return (`KismetMathLibrary.MakeVector` (.x (+ (* (`KismetMathLibrary.ProjectVectorOnToVector` (`local.OldVel`) (`PawnMovementComponent.GetLastInputVector` (`self.GetCharacterMovement`))) (`self.KeepMomentum`)) (* (`KismetMathLibrary.Normal` (`KismetMathLibrary.MakeVector` (.x (`local.OldVel`)) (.y (`local.OldVel`)))) (`self.AirBoostStrenght`)))) (.y (+ (* (`KismetMathLibrary.ProjectVectorOnToVector` (`local.OldVel`) (`PawnMovementComponent.GetLastInputVector` (`self.GetCharacterMovement`))) (`self.KeepMomentum`)) (* (`KismetMathLibrary.Normal` (`KismetMathLibrary.MakeVector` (.x (`local.OldVel`)) (.y (`local.OldVel`)))) (`self.AirBoostStrenght`)))) (`self.DoubleJumpVel`))))