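; Gameplay ability that spawns two BP_CloneCharacter decoys, one on each side of the avatar and turned outward from its facing.
; Both spawn tasks pass the avatar's team ID and set it as instigator.
; When the second spawn succeeds, GE_CloneLife is applied to the owner.
; The ability commits on activation, then waits for a State.Clone.End gameplay event to end itself.
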(event `self.K2_ActivateAbilityFromEvent`
  (params (EventData :type "GameplayEventData Structure (by ref)"))
  (bind _returnvalue (`self.GetAvatarActorFromActorInfo`))
  (bind _returnvalue_2 (`Actor.K2_GetActorRotation` _returnvalue))
  (bind _returnvalue_3 (`Actor.K2_GetActorLocation` _returnvalue))
  (bind _asair_shooter_character (cast `AirShooterCharacter` (`self.GetAvatarActorFromActorInfo`) :!pure true))
  (bind _roll (.roll _returnvalue_2))
  (bind _pitch (.pitch _returnvalue_2))
  (bind _yaw (.yaw _returnvalue_2))
  (bind _returnvalue_4 (* (`KismetMathLibrary.GetRightVector` _returnvalue_2) 90.0))
  (`self.K2_CommitAbility`)
  (bind _teamid (message `/Game/Titanfall_3/Data/BPI_Player.GetTeamID` (`self.GetAvatarActorFromActorInfo`)))
  (`GameplayTask_SpawnActor.SpawnActor` null (+ _returnvalue_3 _returnvalue_4) (`KismetMathLibrary.MakeRotator` _roll _pitch (+ _yaw 90.0)) "/Game/Titanfall_3/Pawns/BP_CloneCharacter.BP_CloneCharacter_C" false _teamid _asair_shooter_character
    (:`then`
      (`GameplayTask_SpawnActor.SpawnActor` null (- _returnvalue_3 _returnvalue_4) (`KismetMathLibrary.MakeRotator` _roll _pitch (- _yaw 90.0)) "/Game/Titanfall_3/Pawns/BP_CloneCharacter.BP_CloneCharacter_C" false _teamid _asair_shooter_character
        (:`then`
          (`AbilityTask_WaitGameplayEvent.WaitGameplayEvent` (struct :`TagName` "State.Clone.End") null
            (:`EventReceived`
              (`self.K2_EndAbility`))))
        (:`Success`
          (`self.BP_ApplyGameplayEffectToOwner` "/Game/Titanfall_3/Abilities/Effects/GE_CloneLife.GE_CloneLife_C" 0))))))