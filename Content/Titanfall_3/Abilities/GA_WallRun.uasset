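; Event-triggered wall-run gameplay ability that starts only while the character is falling and ends on a stop event.
; It saves gravity and speed, zeroes gravity, constrains movement to the horizontal plane and adds a camera roll based on wall side.
; After a zero delay, it sets time-interpolated fly speed and adds input along a target-data direction matched to camera facing.
; Ending restores gravity and falling, removes camera and stamina-drain effects, and hops upward unless cancelled.
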(event `self.K2_OnEndAbility`
  (params (bWasCancelled :type Boolean))
  (bind _returnvalue (`self.GetCharacterMovement`))
  (if (`self.bWallRun`)
    (`MovementComponent.SetPlaneConstraintNormal` _returnvalue (0.0 0.0 0.0))
    (set `CharacterMovementComponent.GravityScale` (`self.OldGrav`) _returnvalue)
    (`CharacterMovementComponent.SetMovementMode` (`self.GetCharacterMovement`) "MOVE_Falling" 0)
    (if (not bWasCancelled)
      (`Character.LaunchCharacter` (`self.GetOwningCharacter`) (0.0 0.0 100.0) false true))
    (set `self.bWallRun` true)
    (`PlayerCameraManager.RemoveCameraModifier` (`PlayerController.PlayerCameraManager` (`Pawn.GetLocalViewingPlayerController` (`self.GetOwningCharacter`))) (`self.CamModReal`))
    (`self.BP_RemoveGameplayEffectFromOwnerWithGrantedTags` (struct :`GameplayTags` (struct :`(TagName` "Gameplay.Effect.StaminaDrain"))))))

(event `self.K2_ActivateAbilityFromEvent`
  (params (EventData :type "GameplayEventData Structure (by ref)"))
  (bind (_eventtag _instigator _target _optionalobject _optionalobject2 _contexthandle _instigatortags _targettags _eventmagnitude _targetdata) (break `GameplayEventData` EventData))
  (bind _returnvalue (`self.GetCharacterMovement`))
  (`KismetSystemLibrary.PrintString` "ability called" true true (struct :`R` 1.0 :`G` 0.051837 :`B` 0.83281 :`A` 1.0))
  (`AbilityTask_WaitGameplayEvent.WaitGameplayEvent` (struct :`TagName` "Event.ActivateAbility.WallRun.Stop") null
    (:`then`
      (if (`NavMovementInterface.IsFalling` (`self.GetCharacterMovement`))
        (set `self.bWallRun` true)
        (`self.K2_CommitAbility`)
        (bind _returnvalue_2 (`PlayerCameraManager.AddNewCameraModifier` (`PlayerController.PlayerCameraManager` (`Pawn.GetLocalViewingPlayerController` (`self.GetOwningCharacter`))) "/Game/Titanfall_3/CameraModifiers/BP_WallRunCam.BP_WallRunCam_C"))
        (bind _output_get (set `self.CamModReal` _returnvalue_2))
        (set `/Game/Titanfall_3/CameraModifiers/BP_WallRunCam.TargetRoll` (`self.CameraTilt` _targetdata) _output_get)
        (set `self.StartTime` (`KismetSystemLibrary.GetGameTimeInSeconds`))
        (`KismetSystemLibrary.PrintString` "lemme run bro" true true (struct :`R` 0.484595 :`G` 1.0 :`B` 0.673352 :`A` 1.0))
        (`self.OldVars`)
        (set `self.PlayerDirection` (`self.Calculate Player direction` _targetdata))
        (`MovementComponent.SetPlaneConstraintNormal` _returnvalue (0.0 0.0 1.0))
        (set `CharacterMovementComponent.GravityScale` 0.0 _returnvalue)
        (set `CharacterMovementComponent.BrakingDecelerationFlying` 0.0 _returnvalue)
        (`AbilityTask_WaitDelay.WaitDelay` 0.0
          (:`OnFinish`
            (set `CharacterMovementComponent.MaxFlySpeed` (`self.FlySpeedLerp`) (`self.GetCharacterMovement`))
            (`Pawn.AddMovementInput` (`GameplayStatics.GetPlayerCharacter` 0) (`KismetMathLibrary.Normal` (`self.PlayerDirection`)) 1.0 false)))
        (else
          (`KismetSystemLibrary.PrintString` "cant wall run" true true (struct :`R` 1.0 :`G` 0.674199 :`B` 0.000405 :`A` 1.0))
          (`self.K2_EndAbility` :!label _label))))
    (:`EventReceived`
      (`KismetSystemLibrary.PrintString` "recieved" true true (struct :`R` 0.448453 :`G` 1.0 :`B` 0.17366 :`A` 1.0))
      (goto _label))))

(fn `Calculate Player direction`
  (params (HitResult :type "GameplayAbilityTargetDataHandle Structure (by ref)"))
  (returns (PlayerDirection :type "Vector Structure"))
  (bind (_bblockinghit _binitialoverlap _time _distance _location) (`GameplayStatics.BreakHitResult` (`AbilitySystemBlueprintLibrary.GetHitResultFromTargetData` HitResult)))
  (return (* _location (`KismetMathLibrary.SelectInt` 1 -1 (> (`KismetMathLibrary.Dot_VectorVector` _location (`SceneComponent.GetForwardVector` (`/Game/FirstPerson/Blueprints/BP_FirstPersonCharacter.FirstPersonCamera` (cast `/Game/FirstPerson/Blueprints/BP_FirstPersonCharacter` (`self.GetAvatarActorFromActorInfo`) :!pure true)))) 0.0)))))

(fn `CameraTilt`
  (params (HitResult :type "GameplayAbilityTargetDataHandle Structure (by ref)"))
  (returns (TiltAmt :type "Float (double-precision)"))
  (if (> (`KismetMathLibrary.Dot_VectorVector` (`.ImpactNormal` (`GameplayStatics.BreakHitResult` (`AbilitySystemBlueprintLibrary.GetHitResultFromTargetData` HitResult))) (`Actor.GetActorRightVector` (`self.GetAvatarActorFromActorInfo`))) 0.0)
    (return -30.0)
    (else
      (return 30.0))))

(fn `FlySpeedLerp`
  (returns (ReturnValue :type "Float (double-precision)"))
  (return (`KismetMathLibrary.Lerp` (`self.InitalSpeed`) (`self.NewSpeed`) (`KismetMathLibrary.MapRangeClamped` (- (`KismetSystemLibrary.GetGameTimeInSeconds`) (`self.StartTime`)) 0.0 1.5 0.0 1.0))))

(fn `OldVars`
  (bind _returnvalue (`self.GetCharacterMovement`))
  (set `self.OldGrav` (`CharacterMovementComponent.GravityScale` (`self.GetCharacterMovement`)))
  (set `self.InitalSpeed` (`KismetMathLibrary.VSize` (`MovementComponent.Velocity` (`self.GetCharacterMovement`))))
  (set `self.OldFly` (`CharacterMovementComponent.BrakingDecelerationFlying` _returnvalue))
  (set `self.Old Fly` (`CharacterMovementComponent.MaxFlySpeed` _returnvalue)))