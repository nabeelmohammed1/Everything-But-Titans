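; Grapple gameplay ability that pulls the avatar toward a surface hit by an instant single-line trace within grapple range.
; A hit adds a cable cue and applies a flying root-motion move, timed by distance over strength, keeping velocity afterward.
; Input release, move completion or a polled proximity check ends it; a miss plays a fail cue, then ends after a short delay.
; On end, the authority commits cooldown and removes the cable cue.
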(event `Debug`
  (`KismetSystemLibrary.DrawDebugSphere` (`self.End Location`) 100.0 12 (struct :`G` 0.066518 :`B` 1.0 :`A` 1.0) 100.0))

(event `self.K2_ActivateAbility`
  (`AbilityTask_WaitInputRelease.WaitInputRelease` false
    (:`then`
      (bind (_asynctaskproxy _data) (`AbilityTask_WaitTargetData.WaitTargetData` "None" "Instant" "/Script/GameplayAbilities.GameplayAbilityTargetActor_SingleLineTrace" (`self.Grapple Distance`) (struct :`Name` "BlockAll") true (`self.MakeTargetLocationInfoFromOwnerActor`) (struct) "/Script/GameplayAbilities.GameplayAbilityWorldReticle" (struct) true)
        (:`ValidData`
          (if (`GameplayStatics.BreakHitResult` (`AbilitySystemBlueprintLibrary.GetHitResultFromTargetData` _data))
            (bind _returnvalue (`AbilitySystemBlueprintLibrary.GetTargetDataEndPoint` _data))
            (set `self.End Location` _returnvalue)
            (`self.K2_AddGameplayCueWithParams` (struct :`TagName` "GameplayCue.Grapple.Cable") (`AbilitySystemBlueprintLibrary.MakeGameplayCueParameters` 0.0 0.0 (struct) (struct) (struct) (struct) (struct) (`self.End Location`)))
            (`|ExecutionSequence`
              (:`then_0`
                (`self.Debug`)
                (`AbilityTask_ApplyRootMotionMoveToForce.ApplyRootMotionMoveToForce` "None" (`self.End Location`) (/ (`KismetMathLibrary.Vector_Distance` (`self.End Location`) (`Actor.K2_GetActorLocation` (`self.GetAvatarActorFromActorInfo`))) (`self.Grapaple Strenght`)) true "MOVE_Flying" false null "MaintainLastRootMotionVelocity"
                  (:`OnTimedOutAndDestinationReached`
                    (`self.K2_EndAbility`))))
              (:`then_1`
                (if (< (`KismetMathLibrary.Vector_Distance` (`self.End Location`) (`Actor.K2_GetActorLocation` (`self.GetAvatarActorFromActorInfo`))) 100.0) :!label _label
                  (`self.K2_EndAbility`)
                  (else
                    (`KismetSystemLibrary.Delay` 0.1)
                    (goto _label)))))
            (else
              (set `self.End Location` _returnvalue)
              (`self.GrappleFail`))))))
    (:`OnRelease`
      (`self.K2_EndAbility`))))

(event `self.K2_OnEndAbility`
  (params (bWasCancelled :type Boolean))
  (`self.K2_HasAuthority`
    (:`True`
      (`self.K2_CommitAbilityCooldown` false)
      (`self.K2_RemoveGameplayCue` (struct :`TagName` "GameplayCue.Grapple.Cable")))))

(event `GrappleFail`
  (`self.K2_AddGameplayCueWithParams` (struct :`TagName` "GameplayCue.Grapple.Fail") (`AbilitySystemBlueprintLibrary.MakeGameplayCueParameters` 0.0 0.0 (struct) (struct) (struct) (struct) (struct) (`self.End Location`)))
  (`KismetSystemLibrary.Delay` 0.5)
  (`self.K2_EndAbility`))