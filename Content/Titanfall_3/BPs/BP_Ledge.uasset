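; Grapple ledge that snaps a flying shooter character onto the nearest landing point when it enters the box.
; BeginPlay caches world locations of components tagged "Grapple"; on overlap it activates GA_RemoveGrapple and picks the closest cached point.
; The authority teleports the character there, draws a debug box and clears the Triggered lock after a short delay.
; VectorPoint and NearestDistanceCheck are helpers the event graph never calls.
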(event `self.ReceiveBeginPlay`
  (`self.SetupArray`))

(event `self.Box.OnComponentBeginOverlap`
  (params (OverlappedComponent :type "PrimitiveComponent Object Reference") (OtherActor :type "Actor Object Reference") (OtherComp :type "PrimitiveComponent Object Reference") (OtherBodyIndex :type Integer) (bFromSweep :type Boolean) (SweepResult :type "HitResult Structure (by ref)"))
  (bind _asbp_shooter_character (cast `/Game/Titanfall_3/GameData/BP_ShooterCharacter` OtherActor :!pure true))
  (bind _output (`|GetArrayItem` (`self.LocationArray`) (`self.index`)))
  (if (`NavMovementComponent.IsFlying` (`Character.CharacterMovement` _asbp_shooter_character))
    (if (not (`self.bTriggered?`))
      (set `self.bTriggered?` true)
      (set `self.nearstdist` 99999.0)
      (`AbilitySystemComponent.K2_GiveAbilityAndActivateOnce` (`AbilitySystemBlueprintLibrary.GetAbilitySystemComponent` OtherActor) "/Game/Titanfall_3/Abilities/GA_RemoveGrapple.GA_RemoveGrapple_C" 0 -1)
      (for (_array_element _array_index) (`self.LocationArray`)
        (bind _returnvalue (`KismetMathLibrary.VSize` (- _array_element (`self.K2_GetActorLocation` OtherActor))))
        (if (< _returnvalue (`self.nearstdist`))
          (set `self.index` _array_index)
          (set `self.nearstdist` _returnvalue)))
      (`/Engine/EditorBlueprintResources/ActorMacros.Switch Has Authority`
        (:`Authority`
          (`/Game/Titanfall_3/GameData/BP_ShooterCharacter.ServerTeleportTo` _asbp_shooter_character _output)
          (`KismetSystemLibrary.DrawDebugBox` _output (50.0 50.0 50.0) (struct :`R` 1.0 :`G` 0.241522 :`B` 0.575345 :`A` 1.0) (struct) 10.0)
          (`KismetSystemLibrary.Delay` 0.4)
          (set `self.bTriggered?` false))))))

(fn `NearestDistanceCheck`
  (params (ArrayVector :type "Vector Structure") (ArrayIndex :type Integer) (`Player Loc` :type "Vector Structure"))
  (bind _returnvalue (`KismetMathLibrary.VSize` (- ArrayVector `Player Loc`)))
  (if (< _returnvalue (`self.nearstdist`))
    (set `self.index` ArrayIndex)
    (set `self.nearstdist` _returnvalue)))

(fn `SetupArray`
  (for _array_element (`self.GetComponentsByTag` "/Script/Engine.SceneComponent" "Grapple")
    (`KismetArrayLibrary.Array_Add` (`self.LocationArray`) (`SceneComponent.K2_GetComponentLocation` _array_element))))

(fn `UserConstructionScript`)

(fn `VectorPoint`
  (params (Actor :type "Actor Object Reference"))
  (returns (ReturnValue :type "Vector Structure"))
  (bind (_returnvalue_x _returnvalue_y) (`KismetMathLibrary.BreakVector` (`self.K2_GetActorLocation` Actor)))
  (bind (_returnvalue_x_2 _returnvalue_y_2 _returnvalue_z) (`KismetMathLibrary.BreakVector` (`self.K2_GetActorLocation` self)))
  (bind (_returnvalue_x_3 _returnvalue_y_3 _returnvalue_z_2) (`KismetMathLibrary.BreakVector` (`BoxComponent.GetScaledBoxExtent` (`self.Box`))))
  (return (`KismetMathLibrary.MakeVector` (`KismetMathLibrary.FClamp` _returnvalue_x (- _returnvalue_x_2 _returnvalue_x_3) (+ _returnvalue_x_2 _returnvalue_x_3)) (`KismetMathLibrary.FClamp` _returnvalue_y (- _returnvalue_y_2 _returnvalue_y_3) (+ _returnvalue_y_2 _returnvalue_y_3)) (+ _returnvalue_z _returnvalue_z_2 150.0))))