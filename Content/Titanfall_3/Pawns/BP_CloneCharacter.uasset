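; BP_CloneCharacter is a clone pawn that walks forward every tick until its active state ends.
; On BeginPlay it applies GE_CloneLife to itself through GAS and starts async listeners.
; An attribute change removes effects tagged State.Clone.Active from the instigator's ability system.
; Losing that tag on the clone itself destroys it, while the State.Clone.End event only prints debug text.
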(event `self.ReceiveBeginPlay`
  (`AbilitySystemComponent.BP_ApplyGameplayEffectToSelf` :`self` (`self.AbilitySystemComponent`) :`GameplayEffectClass` "/Game/Titanfall_3/Abilities/Effects/GE_CloneLife.GE_CloneLife_C" :`Level` 2.0)
  (`AbilityAsync_WaitAttributeChanged.WaitForAttributeChanged` null (struct :`AttributeName` "Health" :`Attribute` "/Script/AirShooter.AirAttributes:Health" :`AttributeOwner` "/Script/CoreUObject.Class'/Script/AirShooter.AirAttributes'")
    (:`then`
      (`AbilityAsync_WaitGameplayTagRemoved.WaitGameplayTagRemoveFromActor` self (struct :`TagName` "State.Clone.Active")
        (:`then`
          (`AbilityAsync_WaitGameplayEvent.WaitGameplayEventToActor` null (struct :`TagName` "State.Clone.End")
            (:`EventReceived`
              (`KismetSystemLibrary.PrintString` "ended"))))
        (:`Removed`
          (`KismetSystemLibrary.PrintString` "i'm done chief" true true (struct :`R` 1.0 :`G` 0.154737 :`B` 0.365291 :`A` 1.0))
          (`self.K2_DestroyActor`))))
    (:`Changed`
      (`KismetSystemLibrary.PrintString` "hit" true true (struct :`R` 1.0 :`G` 0.829919 :`A` 1.0))
      (`AbilitySystemComponent.RemoveActiveEffectsWithTags` (`AbilitySystemBlueprintLibrary.GetAbilitySystemComponent` (`self.GetInstigator`)) (struct :`GameplayTags` (struct :`(TagName` "State.Clone.Active")))))))

(event `self.ReceiveTick`
  (params (DeltaSeconds :type "Float (single-precision)"))
  (`self.AddMovementInput` self (`self.GetActorForwardVector`) 1.0 false))

(fn `UserConstructionScript`)