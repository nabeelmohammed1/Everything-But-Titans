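; Lobby game mode that seats connected players on platforms and tracks whether everyone is ready.
; BeginPlay collects platforms by index tag; logins and logouts wait for that setup, then spawn uniquely colored characters or clear vacated platforms.
; Login also starts voice chat, retrying on short delays until pawns exist, then multicasting VOIP initialization.
; Player info updates refresh the lobby character and pass the all-ready state to the first controller's lobby UI.
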(event `self.ReceiveBeginPlay`
  (`self.SetupPlatforms`))

(event `self.K2_PostLogin`
  (params (NewPlayer :type "PlayerController Object Reference"))
  (`KismetArrayLibrary.Array_Add` (`self.PCs`) NewPlayer)
  (`self.isPlatformSetupDone` :!label _label
    (:`true`
      (`self.UpdatePlatforms`)
      (`self.StarVocie` NewPlayer))))

(event `self.K2_OnLogout`
  (params (ExitingController :type "Controller Object Reference"))
  (bind _asplayer_controller (cast `PlayerController` ExitingController))
  (`KismetArrayLibrary.Array_RemoveItem` (`self.PCs`) _asplayer_controller)
  (goto _label))

(event `StarVocie`
  (params (PC :type "PlayerController Object Reference"))
  (bind _aspc_lobby (cast `/Game/Titanfall_3/GameData/LobbyGamemode/PC_Lobby` PC))
  (`/Game/Titanfall_3/GameData/LobbyGamemode/PC_Lobby.Client_ToggleVoiceatStart` _aspc_lobby)
  (`/Engine/EditorBlueprintResources/StandardMacros.IsValid` (`Controller.K2_GetPawn` _aspc_lobby) :!label _label_2
    (:`Is Valid`
      (for _array_element (`GameStateBase.PlayerArray` (`GameplayStatics.GetGameState`))
        (`KismetSystemLibrary.PrintString` (`KismetSystemLibrary.GetDisplayName` _array_element))
        (bind _returnvalue (`Controller.K2_GetPawn` (`PlayerState.GetPlayerController` _array_element)))
        (`/Engine/EditorBlueprintResources/StandardMacros.IsValid` _returnvalue :!label _label_3
          (:`Is Valid`
            (bind _asbp_lobby_char (cast `/Game/Titanfall_3/GameData/LobbyGamemode/LobbyData/BP_LobbyChar` _returnvalue)
              (:`then`
                (`/Game/Titanfall_3/GameData/LobbyGamemode/LobbyData/BP_LobbyChar.Mulitcast_InitVOIP` _asbp_lobby_char))
              (:`CastFailed`
                (`KismetSystemLibrary.PrintString` (`KismetSystemLibrary.GetDisplayName` _returnvalue)))))
          (:`Is Not Valid`
            (`KismetSystemLibrary.RetriggerableDelay` 0.2)
            (goto _label_3)))))
    (:`Is Not Valid`
      (`KismetSystemLibrary.RetriggerableDelay` 0.2)
      (goto _label_2))))

(fn `CheckifEveryoneisReady`
  (locals (bAllReady :type Boolean))
  (set `local.bAllReady` true)
  (for _array_element (`self.PCs`)
    (bind _aspc_lobby (cast `/Game/Titanfall_3/GameData/LobbyGamemode/PC_Lobby` _array_element))
    (if (not (`.bReady_10_431D78B3435D08419461158DF3E4A321` (break `/Game/Titanfall_3/GameData/LobbyGamemode/LobbyData/S_PlayerLobbyInfo` (`/Game/Titanfall_3/GameData/LobbyGamemode/PC_Lobby.PlayerLobbyInfo_PC` _aspc_lobby))))
      (set `local.bAllReady` false)))
  (bind _aspc_lobby_2 (cast `/Game/Titanfall_3/GameData/LobbyGamemode/PC_Lobby` (`GameplayStatics.GetPlayerController` 0)))
  (set `/Game/Titanfall_3/UI/Lobby/WBP_Lobby.bEnoughPlayersReady` (`local.bAllReady`) (`/Game/Titanfall_3/GameData/LobbyGamemode/PC_Lobby.LobbyUI` _aspc_lobby_2)))

(fn `SetupPlatforms`
  (bind _outactors (`GameplayStatics.GetAllActorsOfClass` "/Game/Titanfall_3/GameData/LobbyGamemode/LobbyData/BP_PlayerPlatform.BP_PlayerPlatform_C"))
  (for _index (range (+ (`KismetArrayLibrary.Array_LastIndex` _outactors) 1))
    (bind _outactors_2 (`GameplayStatics.GetAllActorsOfClassWithTag` "/Game/Titanfall_3/GameData/LobbyGamemode/LobbyData/BP_PlayerPlatform.BP_PlayerPlatform_C" (`KismetStringLibrary.Conv_StringToName` (`KismetStringLibrary.Conv_IntToString` _index))))
    (`KismetArrayLibrary.Array_Add` (`self.PlayerPlatforms`) (`|GetArrayItem` _outactors_2)))
  (set `self.bPlatformsFound` true))

(fn `UpdatePlatforms`
  (locals (bPlayerAlreadyAdded :type Boolean))
  ; Checking if the player was already added
  (for (_array_element _array_index) (`self.PCs`)
    (set `local.bPlayerAlreadyAdded` false)
    (for _array_element_2 (`self.PlayerPlatforms`)
      (if (== (`/Game/Titanfall_3/GameData/LobbyGamemode/LobbyData/BP_PlayerPlatform.PC` _array_element_2) _array_element)
        (set `local.bPlayerAlreadyAdded` true)
        (break)))
    ; Add PC to platform
    (if (not (`local.bPlayerAlreadyAdded`))
      (for _array_element_3 (`self.PlayerPlatforms`)
        (`/Engine/EditorBlueprintResources/StandardMacros.IsValid` (`/Game/Titanfall_3/GameData/LobbyGamemode/LobbyData/BP_PlayerPlatform.PC` _array_element_3)
          (:`Is Not Valid`
            (`/Game/Titanfall_3/GameData/LobbyGamemode/LobbyData/BP_PlayerPlatform.SpawnActor` _array_element_3 _array_element (select `int` _array_index :`0` (struct :`R` 1.0 :`G` 1.0 :`B` 1.0 :`A` 1.0) :`1` (struct :`R` 1.0 :`G` 0.870238 :`B` 0.175347 :`A` 1.0) :`2` (struct :`R` 0.262153 :`G` 1.0 :`B` 0.281913 :`A` 1.0) :`3` (struct :`R` 0.59908 :`G` 0.467014 :`B` 1.0 :`A` 1.0) :`4` (struct :`R` 1.0 :`G` 0.251736 :`B` 0.39817 :`A` 1.0) :`5` (struct :`R` 1.0 :`G` 0.674199 :`B` 0.000405 :`A` 1.0) :`6` (struct :`G` 0.651042 :`B` 0.399086 :`A` 1.0) :`7` (struct :`R` 0.416409 :`G` 1.0 :`B` 0.314732 :`A` 1.0) :`8` (struct :`R` 1.0 :`G` 0.511593 :`B` 0.185764 :`A` 1.0) :`9` (struct :`R` 1.0 :`G` 0.274842 :`B` 0.230903 :`A` 1.0) :!type "LinearColor Structure"))
            (`/Game/Titanfall_3/GameData/LobbyGamemode/LobbyData/BP_PlayerPlatform.VFX Spawn` _array_element_3)
            (break))))))
  ;[0.15 0.02526 0.02526 0.5] Remove PC if disconnected
  (for _array_element_4 (`self.PlayerPlatforms`)
    (if (not (`KismetArrayLibrary.Array_Contains` (`self.PCs`) (`/Game/Titanfall_3/GameData/LobbyGamemode/LobbyData/BP_PlayerPlatform.PC` _array_element_4)))
      (`/Game/Titanfall_3/GameData/LobbyGamemode/LobbyData/BP_PlayerPlatform.Clear` _array_element_4))))

(fn `UpdatePlayerInfo`
  (params (`Requesting Contorller` :type "PlayerController Object Reference"))
  (bind _aspc_lobby (cast `/Game/Titanfall_3/GameData/LobbyGamemode/PC_Lobby` (`local.Requesting Contorller`) :!pure true))
  (bind (_pc _playername _bready) (break `/Game/Titanfall_3/GameData/LobbyGamemode/LobbyData/S_PlayerLobbyInfo` (`/Game/Titanfall_3/GameData/LobbyGamemode/PC_Lobby.PlayerLobbyInfo_PC` _aspc_lobby)))
  (for _array_element (`self.PlayerPlatforms`)
    (if (== (`/Game/Titanfall_3/GameData/LobbyGamemode/LobbyData/BP_PlayerPlatform.PC` _array_element) `Requesting Contorller`)
      (bind _asbp_lobby_char (cast `/Game/Titanfall_3/GameData/LobbyGamemode/LobbyData/BP_LobbyChar` (`/Game/Titanfall_3/GameData/LobbyGamemode/LobbyData/BP_PlayerPlatform.Charcter` _array_element)))
      (`/Game/Titanfall_3/GameData/LobbyGamemode/LobbyData/BP_LobbyChar.UpdatePlayerInfo` _asbp_lobby_char (make `/Game/Titanfall_3/GameData/LobbyGamemode/LobbyData/S_PlayerLobbyInfo` null _playername _bready))
      (`self.CheckifEveryoneisReady`)
      (return)))
  (`/Game/Titanfall_3/GameData/LobbyGamemode/PC_Lobby.TryUpdatingAgain` _aspc_lobby))

(fn `UserConstructionScript`)