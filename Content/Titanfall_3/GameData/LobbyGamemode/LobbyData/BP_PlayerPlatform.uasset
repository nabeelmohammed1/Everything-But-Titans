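; BP_PlayerPlatform is a lobby platform that displays a player's character.
; SpawnActor plays a Niagara ring effect, stores the player controller, and replaces any existing character with a new BP_LobbyChar at the spawn direction transform, passing in a colour value.
; The ring effect destroys itself when finished.
; Clear releases the controller reference and destroys the character.
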(event `SpawnActor`
  (params (PC :type "PlayerController Object Reference") (ColourVal :type "LinearColor Structure"))
  (bind _charcter (`self.Charcter`))
  (bind _returnvalue (`NiagaraFunctionLibrary.SpawnSystemAttached` "/Game/Titanfall_3/VFX/NS_Ring.NS_Ring" (`self.Ring Spawn`) "None" (0.0 0.0 0.0) (struct) "KeepRelativeOffset"))
  (add `NiagaraComponent.OnSystemFinished` _returnvalue (delegate `CustomEvent`))
  (set `self.PC` PC)
  (`/Engine/EditorBlueprintResources/StandardMacros.IsValid` _charcter
    (:`Is Valid`
      (`self.K2_DestroyActor` _charcter))
    (:`Is Not Valid`
      _))
  (bind _returnvalue_2 (`|SpawnActorFromClass` "/Game/Titanfall_3/GameData/LobbyGamemode/LobbyData/BP_LobbyChar.BP_LobbyChar_C" (`SceneComponent.K2_GetComponentToWorld` (`self.PlayerSpawnDirection`)) "Undefined" "MultiplyWithRoot" null ColourVal null))
  (set `self.Charcter` _returnvalue_2))

(event `CustomEvent`
  (params (PSystem :type "NiagaraComponent Object Reference"))
  (`ActorComponent.K2_DestroyComponent` PSystem))

(event `Clear`
  (bind _charcter (`self.Charcter`))
  (set `self.PC` null)
  (`/Engine/EditorBlueprintResources/StandardMacros.IsValid` _charcter
    (:`Is Valid`
      (`self.K2_DestroyActor` _charcter)
      (set `self.Charcter` null))))

(fn `UserConstructionScript`)