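; Game mode for the Sumo game that runs last-player-standing rounds within a match.
; PlayerEliminated clears the player's Alive flag in its PlayerState and fires RoundWon when one player remains.
; RoundWon credits the survivor, then after a delay resets either the round or, once the win limit is reached, the whole match.
; Both resets revive and restart players and update GameState round and phase; match reset also destroys pawns and clears wins.
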(event `RoundWon`
  (bind _roundswon (`/Game/Sumo/Blueprints/PlayerState_Sumo.RoundsWon` (`self.As Player State Sumo`)))
  (bind _asgame_state_sumo (cast `/Game/Sumo/Blueprints/GameState_Sumo` (`GameplayStatics.GetGameState`)))
  (set `self.As Game State Sumo` _asgame_state_sumo)
  (for _array_element (`GameStateBase.PlayerArray` (`self.As Game State Sumo`))
    (bind _asplayer_state_sumo (cast `/Game/Sumo/Blueprints/PlayerState_Sumo` _array_element))
    (if (`/Game/Sumo/Blueprints/PlayerState_Sumo.Alive?` _asplayer_state_sumo)
      (set `self.As Player State Sumo` _asplayer_state_sumo)
      (`/Engine/EditorBlueprintResources/StandardMacros.IncrementInt` _roundswon
        (:`  `
          (`KismetSystemLibrary.PrintString` (`KismetStringLibrary.Conv_IntToString` _roundswon))))))
  (if (>= (`/Game/Sumo/Blueprints/PlayerState_Sumo.RoundsWon` (`self.As Player State Sumo`)) (`self.WinsMAx`))
    (`KismetSystemLibrary.Delay` (`self.matchDelay`))
    (`self.Reset Match`)
    (set `/Game/Sumo/Blueprints/GameState_Sumo.MatchPhase` "NewEnumerator3" (`self.As Game State Sumo`))
    (`KismetSystemLibrary.PrintString` (`KismetStringLibrary.Concat_StrStr` "MatchWinner is " (`PlayerState.GetPlayerName` (`self.As Player State Sumo`))) true true (struct :`G` 0.66 :`B` 1.0 :`A` 1.0) (`self.matchDelay`))
    (else
      (`KismetSystemLibrary.Delay` (`self.roundDelay`))
      (`self.ResetRound`)
      (set `/Game/Sumo/Blueprints/GameState_Sumo.MatchPhase` "NewEnumerator2" (`self.As Game State Sumo`)))))

(fn `PlayerEliminated`
  (params (Actor :type "/Game/Sumo/Blueprints/BP_Player_Sumo Object Reference"))
  (locals (LocalPS :type "PlayerState Object Reference") (LocalAlives :type Integer))
  (`|ExecutionSequence`
    (:`then_0`
      (bind _output_get (set `local.LocalPS` (`Pawn.PlayerState` Actor)))
      (bind _asplayer_state_sumo (cast `/Game/Sumo/Blueprints/PlayerState_Sumo` _output_get))
      (set `/Game/Sumo/Blueprints/PlayerState_Sumo.Alive?` false _asplayer_state_sumo))
    (:`then_1`
      (bind _asgame_state_sumo (cast `/Game/Sumo/Blueprints/GameState_Sumo` (`GameplayStatics.GetGameState`)))
      (for _array_element (`GameStateBase.PlayerArray` _asgame_state_sumo)
        (bind _asplayer_state_sumo_2 (cast `/Game/Sumo/Blueprints/PlayerState_Sumo` _array_element))
        (if (`/Game/Sumo/Blueprints/PlayerState_Sumo.Alive?` _asplayer_state_sumo_2)
          (`/Engine/EditorBlueprintResources/StandardMacros.IncrementInt` (`local.LocalAlives`))))
      (if (== (`local.LocalAlives`) 1)
        (`self.RoundWon`)))))

(fn `Reset Match`
  (bind _as_game_state_sumo (`self.As Game State Sumo`))
  (`KismetSystemLibrary.PrintString` "i reset match")
  (bind _asgame_state_sumo (cast `/Game/Sumo/Blueprints/GameState_Sumo` (`GameplayStatics.GetGameState`)))
  (set `self.As Game State Sumo` _asgame_state_sumo)
  (for _array_element (`GameStateBase.PlayerArray` (`self.As Game State Sumo`))
    (bind _asplayer_state_sumo (cast `/Game/Sumo/Blueprints/PlayerState_Sumo` _array_element))
    (set `/Game/Sumo/Blueprints/PlayerState_Sumo.RoundsWon` 0 _asplayer_state_sumo)
    (set `/Game/Sumo/Blueprints/PlayerState_Sumo.Alive?` true _asplayer_state_sumo)
    (bind _returnvalue (`PlayerState.GetPlayerController` _asplayer_state_sumo))
    (bind _returnvalue_2 (`Controller.K2_GetPawn` _returnvalue))
    (`/Engine/EditorBlueprintResources/StandardMacros.IsValid` _returnvalue_2
      (:`Is Valid`
        (`self.K2_DestroyActor` _returnvalue_2)
        (`self.RestartPlayer` _returnvalue))))
  (set `/Game/Sumo/Blueprints/GameState_Sumo.CurrentRound` 1 _as_game_state_sumo)
  (set `/Game/Sumo/Blueprints/GameState_Sumo.MatchPhase` "NewEnumerator1" _as_game_state_sumo))

(fn `ResetRound`
  (bind _as_game_state_sumo (`self.As Game State Sumo`))
  (`KismetSystemLibrary.PrintString` "i reset round")
  (bind _asgame_state_sumo (cast `/Game/Sumo/Blueprints/GameState_Sumo` (`GameplayStatics.GetGameState`)))
  (set `self.As Game State Sumo` _asgame_state_sumo)
  (for _array_element (`GameStateBase.PlayerArray` (`self.As Game State Sumo`))
    (bind _asplayer_state_sumo (cast `/Game/Sumo/Blueprints/PlayerState_Sumo` _array_element))
    (set `/Game/Sumo/Blueprints/PlayerState_Sumo.Alive?` true _asplayer_state_sumo)
    (bind _returnvalue (`PlayerState.GetPlayerController` _asplayer_state_sumo))
    (bind _returnvalue_2 (`Controller.K2_GetPawn` _returnvalue))
    ; Saving the Spectator
    (`KismetSystemLibrary.PrintString` (`KismetSystemLibrary.GetDisplayName` _returnvalue_2))
    (`/Engine/EditorBlueprintResources/StandardMacros.IsValid` _returnvalue_2
      (:`Is Valid`
        (`Controller.UnPossess` _returnvalue)
        (`self.RestartPlayer` _returnvalue))))
  (`/Engine/EditorBlueprintResources/StandardMacros.IncrementInt` (`/Game/Sumo/Blueprints/GameState_Sumo.CurrentRound` _as_game_state_sumo)
    (:`  `
      (set `/Game/Sumo/Blueprints/GameState_Sumo.MatchPhase` "NewEnumerator1" _as_game_state_sumo))))

(fn `UserConstructionScript`)